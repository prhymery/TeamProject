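; Gun actor shared by players and enemies that aims along a predicted arc and fires team-colored bullets.
; Tick debug-draws the predicted path (for players only while GuideLine is on), moves TargetPoint to the hit's trace end and classifies targets by Player/Tile tags.
; For enemy owners, that result feeds the AIC_Enemy blackboard.
; Shoot spawns a red or blue bullet by owner tag; its SetDelay call is empty.
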(event Custom|SetDelay)

(event EventTick
  (params (DeltaSeconds :type Float%20%28single-precision%29))
  ;[1 1 1] Player Guide line 설정 부분
  (Utilities|Casting|CastToBP_Player_Merging (Components|GetOwner)
    (:then
      (if (Variables|Default|GetGuideLine)
        (Rendering|SetVisibility (Variables|Default|GetTargetPoint) true false)
        ;[1 1 1] 궤적 그리는 부분
        (bind _output_get (Variables|Default|SetShootTransform (Math|Transform|MakeTransform (Transformation|GetWorldLocation (Variables|Default|GetShootPoint)) (Transformation|GetActorRotation (Components|GetOwner))) :!label _label))
        (bind _output_get_2 (Variables|Default|SetDirection (Math|Transform|TransformDirection _output_get (Variables|Default|GetVelocityVector))))
        (bind _outhit (Class|GameplayStatics|BlueprintPredictProjectilePathbyTraceChannel (Transformation|GetWorldLocation (Variables|Default|GetShootPoint)) _output_get_2 true 5.0 "ECC_WorldDynamic" false (Utilities|Array|MakeArray self (Components|GetOwner)) "ForOneFrame" 5.0 3e+01))
        ;[1 1 1] 인식 타겟 포인트 설정
        (Utilities|IsValid (.HitActor (Collision|BreakHitResult _outhit))
          (:Is%20Valid
            (Transformation|SetWorldLocation (Variables|Default|GetTargetPoint) (.TraceEnd (Collision|BreakHitResult _outhit)) false false)
            (if (Actor|ActorHasTag (.HitActor (Collision|BreakHitResult _outhit)) (Utilities|Name|MakeLiteralName "Player"))
              (Variables|Default|SetFocusOnTarget "NewEnumerator1")
              (elif (Actor|ActorHasTag (.HitActor (Collision|BreakHitResult _outhit)) (Utilities|Name|MakeLiteralName "Tile"))
                (Variables|Default|SetFocusOnTarget "NewEnumerator2")
                (else
                  (Variables|Default|SetFocusOnTarget "NewEnumerator0"))))
            (bind _asbp_enemy_c (Utilities|Casting|CastToBP_Enemy_C (Components|GetOwner)))
            (bind _asaic_enemy_c (Utilities|Casting|CastToAIC_Enemy_C (AI|GetAIController _asbp_enemy_c)))
            (Default|SetBlackboardValues _asaic_enemy_c (Variables|Default|GetFocusOnTarget) (.HitActor (Collision|BreakHitResult _outhit)))))
        (else
          (Rendering|SetVisibility (Variables|Default|GetTargetPoint) false false))))
    (:CastFailed
      (goto _label))))

(fn ConstructionScript)

(fn Shoot
  (params (GunOwner :type Actor%20Object%20Reference))
  (bind _returnvalue (Components|GetOwner))
  (bind _shootpoint (Variables|Default|GetShootPoint))
  (bind _returnvalue_2 (Transformation|GetActorRotation _returnvalue))
  (bind _returnvalue_3 (Transformation|GetWorldLocation _shootpoint))
  (bind _returnvalue_4 (Math|Transform|MakeTransform _returnvalue_3 _returnvalue_2 "0.100000,0.100000,0.100000"))
  (if (Actor|ActorHasTag GunOwner "Red")
    (Game|SpawnActorfromClass "/Game/LeeChangJae/Blueprints/BP_Bullet_Red.BP_Bullet_Red_C" _returnvalue_4 "Undefined" 0 0)
    (else
      (Game|SpawnActorfromClass "/Game/LeeChangJae/Blueprints/BP_Bullet_Blue.BP_Bullet_Blue_C" _returnvalue_4 "Undefined" 0 0)))
  (CallFunction|SetDelay))