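; Enemy AI controller that runs a behavior tree and feeds perception results into its blackboard.
; Successfully sensed actors without the Enemy tag set TargetActor when seen, while other senses record the stimulus location as TargetLocation.
; A SetBlackboardValues event lets callers set the ShootingTarget enum, also storing the passed actor as TargetTile for one specific enum value.
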(event OnTargetPerceptionUpdated(AIPerception)
  (params (Actor :type Actor%20Object%20Reference) (Stimulus :type AI%20Stimulus%20Structure))
  (bind (_age _expirationage _strength _stimuluslocation _receiverlocation _tag _bsuccessfullysensed) (Utilities|Struct|BreakAIStimulus Stimulus))
  (if _bsuccessfullysensed
    (if (not (Actor|ActorHasTag Actor "Enemy"))
      (bind _returnvalue (Class|AIPerceptionSystem|GetSenseClassforStimulus Stimulus))
      (if (== _returnvalue "/Script/AIModule.AISense_Sight")
        (AI|Components|Blackboard|SetValueasObject (Variables|Default|GetBlackboard) (Utilities|Name|MakeLiteralName "TargetActor") Actor)
        (else
          (AI|Components|Blackboard|SetValueasVector (Variables|Default|GetBlackboard) (Utilities|Name|MakeLiteralName "TargetLocation") _stimuluslocation))))))

(event Custom|SetBlackboardValues
  (params (ShootingTarget :type Enum_ShootingTarget_Merging%20Enum :default "NewEnumerator0") (TargetActor :type Actor%20Object%20Reference))
  (bind _blackboard (Variables|Default|GetBlackboard))
  (AI|Components|Blackboard|SetValueasEnum _blackboard (Utilities|Name|MakeLiteralName "ShootingTarget") ShootingTarget)
  (if (Utilities|Enum|Equal(Enum) ShootingTarget "NewEnumerator2")
    (AI|Components|Blackboard|SetValueasObject _blackboard (Utilities|Name|MakeLiteralName "TargetTile") TargetActor)))

(event EventBeginPlay
  (AI|RunBehaviorTree (Variables|Default|GetBTAsset)))

(fn ConstructionScript)