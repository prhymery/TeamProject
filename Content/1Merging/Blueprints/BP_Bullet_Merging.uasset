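; BP_Bullet_Merging is a bullet that damages characters whose red or non-red side differs from its own.
; On sphere overlap with a BP_Character_merging, it sets HasRedTag if it is a BP_RedBullet_Merging, found by casting itself.
; It then compares that flag with the character's "Red" actor tag.
; On a mismatch, only the authority calls Damage on the character and destroys the bullet.
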(event OnComponentBeginOverlap(Sphere)
  (params (OverlappedComponent :type Primitive%20Component%20Object%20Reference) (OtherActor :type Actor%20Object%20Reference) (OtherComp :type Primitive%20Component%20Object%20Reference) (OtherBodyIndex :type Integer) (bFromSweep :type Boolean) (SweepResult :type Hit%20Result%20Structure%20%28by%20ref%29))
  (bind _asbp_character_merging (Utilities|Casting|CastToBP_Character_merging OtherActor))
  (Utilities|FlowControl|Sequence
    (:then_0
      (Utilities|Casting|CastToBP_RedBullet_Merging self)
      (Variables|Default|SetHasRedTag true))
    (:then_1
      (if (!= (Variables|Default|GetHasRedTag) (Actor|ActorHasTag _asbp_character_merging "Red"))
        (Networking|SwitchHasAuthority
          (:Authority
            (Default|Damage _asbp_character_merging)
            (Actor|DestroyActor)))))))

(fn ConstructionScript)