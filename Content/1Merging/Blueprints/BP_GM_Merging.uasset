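; Game mode for a Red-versus-Blue "Merging" match that spawns players, gates readiness and announces the winner.
; New players alternate between teams via FlipFlop and possess a character at a random team-tagged PlayerStart, as do respawns.
; Tick flags every controlled character game-ready while AllReady equals PlayerNumber.
; A fixed 30-second timer from BeginPlay, independent of readiness, calls CheckWinColor and shows the Red, Blue or draw widget.
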(event Custom|RespawnPlayer
  (params (PC :type Player%20Controller%20Object%20Reference) (IsRed :type Boolean))
  (Utilities|IsValid PC
    (:Is%20Valid
      (if IsRed
        (bind _outactors (Actor|GetAllActorsOfClasswithTag "/Script/Engine.PlayerStart" "RedStart"))
        (Variables|Default|SetSpawnTransform (Transformation|GetActorTransform (.OutItem (Utilities|Array|Random _outactors))))
        (else
          (bind _outactors_2 (Actor|GetAllActorsOfClasswithTag "/Script/Engine.PlayerStart" "BlueStart"))
          (Variables|Default|SetSpawnTransform (Transformation|GetActorTransform (.OutItem (Utilities|Array|Random _outactors_2))))))
      (bind _returnvalue (Game|SpawnActorfromClass "/Game/1Merging/Blueprints/BP_Character_merging.BP_Character_merging_C" (Variables|Default|GetSpawnTransform) "AlwaysSpawn" 0 0))
      (Utilities|IsValid _returnvalue
        (:Is%20Valid
          (Pawn|Possess PC _returnvalue))))))

(event EventBeginPlay
  (Utilities|FlowControl|Delay 3e+01)
  (bind _returnvalue (Class|ProjectSplashGameModeBase|CheckWinColor))
  (switch Utilities|FlowControl|Switch|SwitchonTileColor _returnvalue
    (:TE_Default
      (bind _returnvalue_2 (UserInterface|CreateWidget "/Game/KoSiHoon/Widgets/UMG_Draw.UMG_Draw_C"))
      (UserInterface|Viewport|AddtoViewport _returnvalue_2 0))
    (:TE_Blue
      (bind _returnvalue_3 (UserInterface|CreateWidget "/Game/KoSiHoon/Widgets/UMG_BlueWin.UMG_BlueWin_C"))
      (UserInterface|Viewport|AddtoViewport _returnvalue_3 0))
    (:TE_Red
      (bind _returnvalue_4 (UserInterface|CreateWidget "/Game/KoSiHoon/Widgets/UMG_RedWin.UMG_RedWin_C"))
      (UserInterface|Viewport|AddtoViewport _returnvalue_4 0))))

(event EventTick
  (params (DeltaSeconds :type Float%20%28single-precision%29))
  (if (== (Variables|Default|GetAllReady) (Variables|Default|GetPlayerNumber))
    (bind _outactors (Actor|GetAllActorsOfClass "/Game/1Merging/Blueprints/BP_PC_Merging.BP_PC_Merging_C"))
    (for _array_element _outactors
      (bind _asbp_character_merging (Utilities|Casting|CastToBP_Character_merging (Pawn|GetControlledPawn _array_element)))
      (Variables|/Game/1Merging/Blueprints/BP_Character_merging.BP_Character_merging_C|SetIsGameReady _asbp_character_merging true))))

(event EventHandleStartingNewPlayer
  (params (NewPlayer :type Player%20Controller%20Object%20Reference))
  (Utilities|FlowControl|FlipFlop
    (:A
      (bind _outactors (Actor|GetAllActorsOfClasswithTag "/Script/Engine.PlayerStart" "RedStart"))
      (Variables|Default|SetSpawnTransform (Transformation|GetActorTransform (.OutItem (Utilities|Array|Random _outactors))))
      (bind _returnvalue (Game|SpawnActorfromClass "/Game/1Merging/Blueprints/BP_Character_merging.BP_Character_merging_C" (Math|Transform|MakeTransform (.Location (Math|Transform|BreakTransform (Variables|Default|GetSpawnTransform))) "0, 0, 0" "1.000000,1.000000,1.000000") "AdjustIfPossibleButAlwaysSpawn" NewPlayer 0))
      (Pawn|Possess NewPlayer _returnvalue))
    (:B
      (bind _outactors_2 (Actor|GetAllActorsOfClasswithTag "/Script/Engine.PlayerStart" "BlueStart"))
      (Variables|Default|SetSpawnTransform (Transformation|GetActorTransform (.OutItem (Utilities|Array|Random _outactors_2))))
      (bind _returnvalue_2 (Game|SpawnActorfromClass "/Game/1Merging/Blueprints/BP_Character_merging.BP_Character_merging_C" (Math|Transform|MakeTransform (.Location (Math|Transform|BreakTransform (Variables|Default|GetSpawnTransform))) "0.000000,180.000000,0.000000" "1.000000,1.000000,1.000000") "AdjustIfPossibleButAlwaysSpawn" NewPlayer 0))
      (Pawn|Possess NewPlayer _returnvalue_2))))

(fn ConstructionScript)