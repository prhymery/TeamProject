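; Game state for the Merging game that tracks the match phase (None, Ready, Play, End), play time and result.
; BeginPlay sets Ready, and an authority-only Tick holds PlayTime at zero in None or Ready and accumulates it during Play.
; The CurrentGamestate RepNotify calls GameStart or GameEnd with the result on player controller 0 (BP_PC_Merging).
; SetEndProperty sets the result before the phase.
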(event EventBeginPlay
  (Variables|Default|SetCurrentGamestate "NewEnumerator1"))

(event EventTick
  (params (DeltaSeconds :type Float%20%28single-precision%29))
  (Networking|SwitchHasAuthority
    (:Authority
      (switch Utilities|FlowControl|Switch|SwitchonEnum_CurrentGameState (Variables|Default|GetCurrentGamestate)
        (:NewEnumerator0
          (Variables|Default|SetPlayTime 0.0 :!label _label))
        (:NewEnumerator1
          (goto _label))
        (:NewEnumerator2
          (Variables|Default|SetPlayTime (+ DeltaSeconds (Variables|Default|GetPlayTime))))))))

(fn ConstructionScript)

(fn OnRepCurrentGamestate
  (switch Utilities|FlowControl|Switch|SwitchonEnum_CurrentGameState (Variables|Default|GetCurrentGamestate)
    (:NewEnumerator2
      (CallFunction|DoStart))
    (:NewEnumerator3
      (CallFunction|DoEnd (Variables|Default|GetGameResult)))))

(fn DoStart
  (Default|GameStart (.AsBP%20PC%20Merging (Utilities|Casting|CastToBP_PC_Merging (Game|GetPlayerController 0)))))

(fn DoEnd
  (params (EndGameResult :type TileColor%20Enum :default "TE_Default"))
  (Default|GameEnd (.AsBP%20PC%20Merging (Utilities|Casting|CastToBP_PC_Merging (Game|GetPlayerController 0))) EndGameResult))

(fn SetEndProperty
  (params (GameResult :type TileColor%20Enum :default "TE_Default") (CurrentGamestate :type Enum_CurrentGameState%20Enum :default "NewEnumerator0"))
  (Variables|Default|SetGameResult GameResult)
  (Variables|Default|SetCurrentGamestate CurrentGamestate))