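; Gun Blueprint that handles aim prediction for the player and enemies, showing a trajectory guide and target point.
; Each Tick it predicts a projectile path from the Muzzle socket, debug-draws it and moves TargetPoint on a hit; player-owned guns do this only when GuideLine is on.
; Hits are classified by Player or Tile tag, and enemy-owned guns pass the result and hit actor to their AI controller's blackboard.
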(event Custom|SetDelay)

(event EventTick
  (params (DeltaSeconds :type Float%20%28single-precision%29))
  ;[1 1 1] Player Guide line 설정 부분
  (Utilities|Casting|CastToBP_Player_Merging (Components|GetOwner)
    (:then
      (if (Variables|Default|GetGuideLine)
        (Rendering|SetVisibility (Variables|Default|GetTargetPoint) true false)
        ;[1 1 1] 궤적 그리는 부분
        (bind _output_get (Variables|Default|SetShootTransform (Math|Transform|MakeTransform (Transformation|GetSocketLocation (Variables|Default|GetBody) "Muzzle") (Transformation|GetActorRotation)) :!label _label))
        (bind _output_get_2 (Variables|Default|SetDirection (Math|Transform|TransformDirection _output_get (Variables|Default|GetVelocityVector))))
        (bind _outhit (Class|GameplayStatics|BlueprintPredictProjectilePathbyTraceChannel (Transformation|GetSocketLocation (Variables|Default|GetBody) "Muzzle") _output_get_2 true 5.0 "ECC_WorldDynamic" false (Utilities|Array|MakeArray self (Components|GetOwner)) "ForOneFrame" 5.0 3e+01))
        ;[1 1 1] 인식 타겟 포인트 설정
        (Utilities|IsValid (.HitActor (Collision|BreakHitResult _outhit))
          (:Is%20Valid
            (Transformation|SetWorldLocation (Variables|Default|GetTargetPoint) (.TraceEnd (Collision|BreakHitResult _outhit)) false false)
            (if (Actor|ActorHasTag (.HitActor (Collision|BreakHitResult _outhit)) (Utilities|Name|MakeLiteralName "Player"))
              (Variables|Default|SetFocusOnTarget "NewEnumerator1")
              (elif (Actor|ActorHasTag (.HitActor (Collision|BreakHitResult _outhit)) (Utilities|Name|MakeLiteralName "Tile"))
                (Variables|Default|SetFocusOnTarget "NewEnumerator2")
                (else
                  (Variables|Default|SetFocusOnTarget "NewEnumerator0"))))
            (bind _asbp_enemy_merging (Utilities|Casting|CastToBP_Enemy_Merging (Components|GetOwner)))
            (bind _asaic_enemy_merging (Utilities|Casting|CastToAIC_Enemy_Merging (AI|GetAIController _asbp_enemy_merging)))
            (Default|SetBlackboardValues _asaic_enemy_merging (Variables|Default|GetFocusOnTarget) (.HitActor (Collision|BreakHitResult _outhit)))))
        (else
          (Rendering|SetVisibility (Variables|Default|GetTargetPoint) false false))))
    (:CastFailed
      (goto _label))))

(fn ConstructionScript)