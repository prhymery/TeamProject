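; HUD Blueprint that creates the match's on-screen widgets: minimap, world map, ready screen and end-game results.
; BeginPlay adds a visible minimap and a world map that starts hidden because the minimap is visible.
; It then reads CurrentGamestate from BP_GameState_Merging to show the ready widget or remove it during Play.
; The Result event adds a Blue win, Red win or Draw widget according to the passed result.
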(event Custom|Result
  (params (EndGameResult :type TileColor%20Enum :default "TE_Default"))
  (switch Utilities|FlowControl|Switch|SwitchonTileColor EndGameResult
    (:TE_Default
      (bind _returnvalue (UserInterface|CreateWidget "/Game/KoSiHoon/Widgets/UMG_Draw.UMG_Draw_C"))
      (UserInterface|Viewport|AddtoViewport _returnvalue 0))
    (:TE_Blue
      (bind _returnvalue_2 (UserInterface|CreateWidget "/Game/KoSiHoon/Widgets/UMG_BlueWin.UMG_BlueWin_C"))
      (UserInterface|Viewport|AddtoViewport _returnvalue_2 0))
    (:TE_Red
      (bind _returnvalue_3 (UserInterface|CreateWidget "/Game/KoSiHoon/Widgets/UMG_RedWin.UMG_RedWin_C"))
      (UserInterface|Viewport|AddtoViewport _returnvalue_3 0))))

(event EventBeginPlay
  (Utilities|FlowControl|Sequence
    (:then_0
      (bind _returnvalue (UserInterface|CreateWidget "/Game/WooSeoHyeon/MiniMap/UI/WBP_MiniMap.WBP_MiniMap_C"))
      (Widget|SetVisibility _returnvalue "Visible")
      (Variables|Default|SetMiniMap _returnvalue)
      (UserInterface|Viewport|AddtoViewport _returnvalue 0))
    (:then_1
      (bind _output_get (Variables|/Script/UMG.Widget|SetVisibility _returnvalue "Visible"))
      (bind _returnvalue_2 (UserInterface|CreateWidget "/Game/WooSeoHyeon/MiniMap/UI/WBP_WorldMap.WBP_WorldMap_C"))
      (Variables|Default|SetWorldMap _returnvalue_2)
      (if (not (Utilities|Enum|Equal(Enum) _output_get "Visible"))
        (Widget|SetVisibility _returnvalue_2 "Visible")
        (UserInterface|Viewport|AddtoViewport _returnvalue_2 0)
        (else
          (Widget|SetVisibility _returnvalue_2 "Hidden")
          (UserInterface|Viewport|AddtoViewport _returnvalue_2 0))))
    (:then_2
      (switch Utilities|FlowControl|Switch|SwitchonEnum_CurrentGameState (Variables|/Game/1Merging/Blueprints/BP_GameState_Merging.BP_GameState_Merging_C|GetCurrentGamestate (.AsBP%20Game%20State%20Merging (Utilities|Casting|CastToBP_GameState_Merging (Game|GetGameState))))
        (:NewEnumerator1
          (bind _returnvalue_3 (UserInterface|CreateWidget "/Game/KoSiHoon/Widgets/UMG_GameReady.UMG_GameReady_C"))
          (bind _output_get_2 (Variables|Default|SetReadyWidget _returnvalue_3))
          (UserInterface|Viewport|AddtoViewport _output_get_2 0))
        (:NewEnumerator2
          (CallFunction|RemoveReadyWidget))))))

(event Collision|EventActorBeginOverlap
  (params (OtherActor :type Actor%20Object%20Reference)))

(event EventTick
  (params (DeltaSeconds :type Float%20%28single-precision%29)))

(fn ConstructionScript)

(fn RemoveReadyWidget
  (bind _readywidget (Variables|Default|GetReadyWidget))
  (Utilities|IsValid _readywidget
    (:Is%20Valid
      (Widget|RemovefromParent _readywidget))))