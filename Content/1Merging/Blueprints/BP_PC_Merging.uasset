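; BP_PC_Merging is a player controller that provides a debug-style chat connection hotkey and a respawn hook.
; Pressing 0 asks MyGameInstance to connect to the chat server and, on success, calls its CreateThread.
; Client_Respawn checks for a valid game mode, casts it to BP_GM_Merging and has it respawn this controller's player.
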(event Custom|Client_Respawn
  (bind _returnvalue (Game|GetGameMode))
  (Utilities|IsValid _returnvalue
    (:Is%20Valid
      (bind _asbp_gm_merging (Utilities|Casting|CastToBP_GM_Merging _returnvalue))
      (Default|RespawnPlayer _asbp_gm_merging self))))

(event Input|KeyboardEvents|0
  (params (Key :type Key%20Structure :default "None"))
  (:Pressed
    (bind _asmy_game_instance (Utilities|Casting|CastToMyGameInstance (Game|GetGameInstance)))
    (bind _returnvalue (Class|MyGameInstance|ConnectChatServer _asmy_game_instance))
    (if _returnvalue
      (Class|MyGameInstance|CreateThread _asmy_game_instance))))

(fn ConstructionScript)