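; Player Blueprint for the Merging game that carries a gun and sends preset chat messages.
; On BeginPlay it spawns BP_Gun_Merging, snaps it to the GunPoint component and stores it as CurrentGun.
; Left mouse fires the gun, and middle mouse toggles its guide line through a FlipFlop.
; Number keys 1 to 4 send Default, Provoke, Good or Bad chat messages through MyGameInstance.
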(event EventBeginPlay
  (bind _self self)
  (|CallParentFunction)
  (bind _returnvalue (Game|SpawnActorfromClass "/Game/1Merging/Blueprints/BP_Gun_Merging.BP_Gun_Merging_C" (Transformation|GetWorldTransform (Variables|Default|GetGunPoint)) "Undefined" _self _self))
  (Variables|Default|SetCurrentGun _returnvalue)
  (Transformation|AttachComponentToComponent _returnvalue (Variables|Default|GetGunPoint) "None" "SnapToTarget" "SnapToTarget" "KeepRelative" true))

(event Input|KeyboardEvents|4
  (params (Key :type Key%20Structure))
  (:Pressed
    (bind _asmy_game_instance (Utilities|Casting|CastToMyGameInstance (Game|GetGameInstance)))
    (Class|MyGameInstance|SendChatting _asmy_game_instance "TE_Bad")))

(event Input|KeyboardEvents|1
  (params (Key :type Key%20Structure))
  (:Pressed
    (bind _asmy_game_instance (Utilities|Casting|CastToMyGameInstance (Game|GetGameInstance)))
    (Class|MyGameInstance|SendChatting _asmy_game_instance "TE_Default")))

(event Input|KeyboardEvents|2
  (params (Key :type Key%20Structure))
  (:Pressed
    (bind _asmy_game_instance (Utilities|Casting|CastToMyGameInstance (Game|GetGameInstance)))
    (Class|MyGameInstance|SendChatting _asmy_game_instance "TE_Provoke")))

(event Input|KeyboardEvents|3
  (params (Key :type Key%20Structure))
  (:Pressed
    (bind _asmy_game_instance (Utilities|Casting|CastToMyGameInstance (Game|GetGameInstance)))
    (Class|MyGameInstance|SendChatting _asmy_game_instance "TE_Good")))

(event Input|MouseEvents|MiddleMouseButton
  (params (Key :type Key%20Structure))
  (bind _currentgun (Variables|Default|GetCurrentGun))
  (:Pressed
    (Utilities|IsValid (Variables|Default|GetCurrentGun)
      (:Is%20Valid
        (bind _isa (Utilities|FlowControl|FlipFlop)
          (:A
            (Variables|/Game/1Merging/Blueprints/BP_Gun_Merging.BP_Gun_Merging_C|SetGuideLine _currentgun _isa))
          (:B
            (Variables|/Game/1Merging/Blueprints/BP_Gun_Merging.BP_Gun_Merging_C|SetGuideLine _currentgun _isa)))))))

(event Input|MouseEvents|LeftMouseButton
  (params (Key :type Key%20Structure))
  (:Pressed
    (Default|Shoot (Variables|Default|GetCurrentGun) self)))

(fn ConstructionScript)