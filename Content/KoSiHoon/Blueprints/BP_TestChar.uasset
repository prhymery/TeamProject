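; BP_TestChar is a test character for trying out projectile and gun spawning, apparently in a networked setup.
; Key 1 calls C2S_Fire, named as a client-to-server event, which spawns a blue test bullet at Arrow1's transform only on authority.
; Key 2 calls C2S_SpawnGun, which spawns a BP_Gun owned by the character at the same arrow and fires it immediately, without an authority check.
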(event Custom|C2S_Fire
  (Networking|SwitchHasAuthority
    (:Authority
      (Game|SpawnActorfromClass "/Game/KoSiHoon/Blueprints/BP_TestBullet_Blue.BP_TestBullet_Blue_C" (Transformation|GetWorldTransform (Variables|Default|GetArrow1)) "Undefined" 0 0))))

(event Custom|C2S_SpawnGun
  (bind _returnvalue (Game|SpawnActorfromClass "/Game/KoSiHoon/Blueprints/BP_Gun.BP_Gun_C" (Transformation|GetWorldTransform (Variables|Default|GetArrow1)) "Undefined" self 0))
  (Class|Gun|Fire _returnvalue))

(event EventBeginPlay)

(event Collision|EventActorBeginOverlap
  (params (OtherActor :type Actor%20Object%20Reference)))

(event EventTick
  (params (DeltaSeconds :type Float%20%28single-precision%29)))

(event Input|KeyboardEvents|2
  (params (Key :type Key%20Structure :default "None"))
  (:Pressed
    (CallFunction|C2SSpawnGun)))

(event Input|KeyboardEvents|1
  (params (Key :type Key%20Structure :default "None"))
  (:Pressed
    (CallFunction|C2SFire)))

(fn ConstructionScript)