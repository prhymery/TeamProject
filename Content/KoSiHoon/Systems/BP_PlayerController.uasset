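; Player controller that hooks up the chat UI and debug-style thread controls through MyGameInstance.
; On BeginPlay it passes UMG_ChattingBox to the game instance and has it load the chat widget.
; The 1 and 2 keys call CreateThread and DeleteThread on the game instance, which owns the actual logic.
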(event EventBeginPlay
  (bind _asmy_game_instance (Utilities|Casting|CastToMyGameInstance (Game|GetGameInstance)))
  (Class|MyGameInstance|SetChattingBox _asmy_game_instance "/Game/KoSiHoon/Widgets/UMG_ChattingBox.UMG_ChattingBox_C")
  (Class|MyGameInstance|LoadChatWidget _asmy_game_instance))

(event EventTick
  (params (DeltaSeconds :type Float%20%28single-precision%29)))

(event Input|KeyboardEvents|1
  (params (Key :type Key%20Structure :default "None"))
  (:Pressed
    (bind _asmy_game_instance (Utilities|Casting|CastToMyGameInstance (Game|GetGameInstance)))
    (Class|MyGameInstance|CreateThread _asmy_game_instance)))

(event Input|KeyboardEvents|2
  (params (Key :type Key%20Structure :default "None"))
  (:Pressed
    (bind _asmy_game_instance (Utilities|Casting|CastToMyGameInstance (Game|GetGameInstance)))
    (Class|MyGameInstance|DeleteThread _asmy_game_instance)))

(fn ConstructionScript)