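; AI controller for Enemy C that starts the BT_Enemy_C behavior tree on BeginPlay and feeds perception results into its blackboard.
; A successfully sensed sight stimulus stores the actor as TargetActor, while any other sense stores the stimulus location as TargetLocation.
; Lost stimuli are ignored, so neither key is cleared here.
; Helper events let callers set named bool keys and the ShootingTarget enum key.
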(event OnTargetPerceptionUpdated(AIPerception)
  (params (Actor :type Actor%20Object%20Reference) (Stimulus :type AI%20Stimulus%20Structure))
  (bind (_age _expirationage _strength _stimuluslocation _receiverlocation _tag _bsuccessfullysensed) (Utilities|Struct|BreakAIStimulus Stimulus))
  (if _bsuccessfullysensed
    (bind _returnvalue (Class|AIPerceptionSystem|GetSenseClassforStimulus Stimulus))
    (if (== _returnvalue "/Script/AIModule.AISense_Sight")
      (AI|Components|Blackboard|SetValueasObject (Variables|Default|GetBlackboard) (Utilities|Name|MakeLiteralName "TargetActor") Actor)
      (else
        (AI|Components|Blackboard|SetValueasVector (Variables|Default|GetBlackboard) (Utilities|Name|MakeLiteralName "TargetLocation") _stimuluslocation)))))

(event Custom|SetBlackboardValueAsBool
  (params (Value :type Boolean) (Name :type Name))
  (AI|Components|Blackboard|SetValueasBool (Variables|Default|GetBlackboard) Name Value))

(event Custom|SetBlackboardValueAsEnum
  (params (ShootingTarget :type Enum_ShootingTarget%20Enum :default "NewEnumerator0"))
  (AI|Components|Blackboard|SetValueasEnum (Variables|Default|GetBlackboard) (Utilities|Name|MakeLiteralName "ShootingTarget") ShootingTarget))

(event EventBeginPlay
  (AI|RunBehaviorTree "/Game/LeeChangJae/Blueprints/AI/BT_Enemy_C.BT_Enemy_C"))

(fn ConstructionScript)