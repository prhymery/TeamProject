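; BP_Bullet is a short-lived bullet actor that makes noise when spawned and destroys itself on impact.
; BeginPlay plays the Collapse01 sound at its location, reports a ranged noise event with itself as instigator for AI hearing, and sets a brief lifespan.
; A Sphere hit prints the other actor's name and destroys the bullet; the Floor tag check has empty branches, and no damage is applied.
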(event OnComponentHit(Sphere)
  (params (HitComponent :type Primitive%20Component%20Object%20Reference) (OtherActor :type Actor%20Object%20Reference) (OtherComp :type Primitive%20Component%20Object%20Reference) (NormalImpulse :type Vector :default "0, 0, 0") (Hit :type Hit%20Result%20Structure%20%28by%20ref%29))
  (Development|PrintString (Utilities|GetDisplayName OtherActor))
  (if (Actor|ActorHasTag OtherActor "Floor")
    _
    (else
      _))
  (Actor|DestroyActor))

(event EventBeginPlay
  (bind _returnvalue (Transformation|GetActorLocation))
  (Audio|PlaySoundatLocation "/Game/StarterContent/Audio/Collapse01.Collapse01" _returnvalue "0, 0, 0" 1.0 1.0 0.0 0 0 0 0)
  (Class|AISenseHearing|ReportNoiseEvent _returnvalue 2.0 self 1e+03 "None")
  (Actor|SetLifeSpan 3.0))

(fn ConstructionScript)