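; BP_Enemy_C is an armed enemy driven by the AIC_Enemy_C AI controller.
; On BeginPlay it hides its Sphere, then spawns a BP_Gun attached to GunPoint with the guide line enabled.
; SetAlerted reveals the Sphere, and CheckFocus forwards its value to the AI controller as a blackboard enum.
; A delay-throttled shooting chain exists in the event graph but is unconnected and never runs.
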(event Custom|SetAlerted
  (Rendering|SetVisibility (Variables|Default|GetSphere) true false))

(event Custom|CheckFocus
  (params (Value :type Enum_ShootingTarget%20Enum :default "NewEnumerator0"))
  (bind _asaic_enemy_c (Utilities|Casting|CastToAIC_Enemy_C (AI|GetAIController self)))
  (Default|SetBlackboardValueasEnum _asaic_enemy_c Value))

(event EventBeginPlay
  (bind _self self)
  (|CallParentFunction)
  (Rendering|SetVisibility (Variables|Default|GetSphere) false false)
  (bind _returnvalue (Game|SpawnActorfromClass "/Game/LeeChangJae/Blueprints/BP_Gun.BP_Gun_C" (Transformation|GetWorldTransform (Variables|Default|GetGunPoint)) "Undefined" _self _self))
  (bind _output_get (Variables|Default|SetCurrentGun _returnvalue))
  (Transformation|AttachComponentToComponent _returnvalue (Variables|Default|GetGunPoint) "None" "SnapToTarget" "SnapToTarget" "KeepRelative" true)
  (Variables|/Game/LeeChangJae/Blueprints/BP_Gun.BP_Gun_C|SetGuideLine _output_get true))

(fn ConstructionScript)