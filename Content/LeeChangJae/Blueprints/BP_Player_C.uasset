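; BP_Player_C is a player Blueprint that equips a gun and handles its input.
; On BeginPlay it runs the parent logic, then spawns a BP_Gun at the GunPoint component, snaps it there and keeps it as CurrentGun.
; Left Ctrl fires the current gun, and the middle mouse button toggles its GuideLine flag through a FlipFlop when the gun is valid.
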(event EventBeginPlay
  (|CallParentFunction)
  (bind _returnvalue (Game|SpawnActorfromClass "/Game/LeeChangJae/Blueprints/BP_Gun.BP_Gun_C" (Transformation|GetWorldTransform (Variables|Default|GetGunPoint)) "Undefined" 0 0))
  (Variables|Default|SetCurrentGun _returnvalue)
  (Transformation|AttachComponentToComponent _returnvalue (Variables|Default|GetGunPoint) "None" "SnapToTarget" "SnapToTarget" "KeepRelative" true))

(event EventTick
  (params (DeltaSeconds :type Float%20%28single-precision%29)))

(event Input|KeyboardEvents|LeftCtrl
  (params (Key :type Key%20Structure :default "None"))
  (:Pressed
    (Default|Shoot (Variables|Default|GetCurrentGun))))

(event Input|MouseEvents|MiddleMouseButton
  (params (Key :type Key%20Structure :default "None"))
  (bind _currentgun (Variables|Default|GetCurrentGun))
  (:Pressed
    (Utilities|IsValid (Variables|Default|GetCurrentGun)
      (:Is%20Valid
        (bind _isa (Utilities|FlowControl|FlipFlop)
          (:A
            (Variables|/Game/LeeChangJae/Blueprints/BP_Gun.BP_Gun_C|SetGuideLine _currentgun _isa))
          (:B
            (Variables|/Game/LeeChangJae/Blueprints/BP_Gun.BP_Gun_C|SetGuideLine _currentgun _isa)))))))

(fn ConstructionScript)