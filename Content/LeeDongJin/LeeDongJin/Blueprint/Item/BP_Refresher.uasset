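; BP_Refresher is an item Actor that spins in place and disappears when the player character touches it.
; Tick applies a yaw rotation scaled by delta time, and the Box overlap destroys the Actor after a cast to BP_ThirdPersonCharacter succeeds.
; Nodes for setting health, updating health and spawning an actor are left disconnected, so pickup has no other effect in this Blueprint.
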(event OnComponentBeginOverlap(Box)
  (params (OverlappedComponent :type Primitive%20Component%20Object%20Reference) (OtherActor :type Actor%20Object%20Reference) (OtherComp :type Primitive%20Component%20Object%20Reference) (OtherBodyIndex :type Integer) (bFromSweep :type Boolean) (SweepResult :type Hit%20Result%20Structure%20%28by%20ref%29))
  (Utilities|Casting|CastToBP_ThirdPersonCharacter OtherActor)
  (Actor|DestroyActor))

(event EventTick
  (params (DeltaSeconds :type Float%20%28single-precision%29))
  (Transformation|AddActorLocalRotation (Math|Rotator|MakeRotator 0.0 0.0 (* (Variables|Default|GetRotation) DeltaSeconds)) false false))

(fn ConstructionScript)