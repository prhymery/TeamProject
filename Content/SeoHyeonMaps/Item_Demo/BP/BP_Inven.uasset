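; BP_Inven is a demo inventory Blueprint that holds a list of item IDs for multiplayer play.
; Server_AddItem passes an ID to AddItem, which appends it to ItemList and calls Multi_PrintDebugString to print every index and ID on screen for debugging.
; GetAllItemString joins the IDs into a comma-separated string.
; ItemList has a RepNotify function, but it is empty, as are BeginPlay and Tick.
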(event Custom|Multi_PrintDebugString
  (CallFunction|PrintAllItem))

(event Custom|Server_AddItem
  (params (ItemID :type Integer))
  (CallFunction|AddItem ItemID))

(event EventBeginPlay)

(event EventTick
  (params (DeltaSeconds :type Float%20%28single-precision%29)))

(fn PrintAllItem
  ;[1 1 1] 모든 아이템 목록 출력 (디버깅용)
  (for (_array_element _array_index) (Variables|Default|GetItemList)
    (Development|PrintString (Utilities|String|Append "Index : " (Utilities|String|ToString(Integer) _array_index) "/ ItemID : " (Utilities|String|ToString(Integer) _array_element)) true true "(R=0.000000,G=0.660000,B=1.000000,A=1.000000)" (Variables|Default|GetDebugStringDuration))))

(fn AddItem
  (params (ItemID :type Integer))
  (Utilities|Array|Add (Variables|Default|GetItemList) ItemID)
  (CallFunction|MultiPrintDebugString))

(fn GetAllItemString
  (for _array_element (Variables|Default|GetItemList)
    (LocalVariables|SetResult (Utilities|String|Append (LocalVariables|GetResult) "," (Utilities|String|ToString(Integer) _array_element))))
  (return (LocalVariables|GetResult)))

(fn OnRepItemList)